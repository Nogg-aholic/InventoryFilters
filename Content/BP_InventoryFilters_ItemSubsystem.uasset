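; Item subsystem Blueprint for InventoryFilters that builds the item records at startup.
; On BeginPlay it polls on a two-second delay until two manager lookups are valid, logged as the Recipe and Schematic managers.
; It then gathers all descriptors through CheatGetAllDescriptors and passes them to RebuildItemRecords.
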(event EventBeginPlay
  (Class|BlueprintLoggingLibrary|LogVerbose "InventoryFilters_ItemSubsystemBP Created")
  (Utilities|FlowControl|Delay 2.0 :!label _label)
  (if (and (Utilities|IsValid (Class|FGRecipeManager|Get)) (Utilities|IsValid (Class|FGSchematicManager|Get)))
    (bind _out_descriptors (Class|FGBlueprintFunctionLibrary|CheatGetAllDescriptors))
    (Class|InventoryFiltersItemSubsystem|RebuildItemRecords _out_descriptors)
    (else
      (Class|BlueprintLoggingLibrary|LogVerbose "InventoryFilters waiting for Recipe and Schematic manager to be ready")
      (goto _label))))

(fn ConstructionScript)